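; Niagara gravity pole effect actor that continually shifts the two user colors of its particle system.
; On BeginPlay, two looping timers, each with a randomized interval, call SetColorA and SetColorB, which store the previous color, pick a random hue and restart their timeline.
; The timelines blend old to new color in HSV space and write the result to the Niagara User.ColorA and User.ColorB parameters.
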(event `self.ReceiveBeginPlay`
  (`parent.ReceiveBeginPlay`)
  (`KismetSystemLibrary.K2_SetTimer` null "SetColorA" (`KismetMathLibrary.RandomFloatInRange` 5.0 10.0) true)
  (`KismetSystemLibrary.K2_SetTimer` null "SetColorB" (`KismetMathLibrary.RandomFloatInRange` 7.0 12.0) true))

(fn `SetColorA`
  (bind _newcolora (`self.NewColorA`))
  (set `self.PreviousColorA` _newcolora)
  (`KismetMathLibrary.LinearColor_SetRandomHue` _newcolora)
  (`TimelineComponent.PlayFromStart` (`self.ColorAInterp`)))

(fn `SetColorB`
  (bind _newcolorb (`self.NewColorB`))
  (set `self.PreviousColorB` _newcolorb)
  (`KismetMathLibrary.LinearColor_SetRandomHue` _newcolorb)
  (`TimelineComponent.PlayFromStart` (`self.ColorBInterp`)))

(fn `UserConstructionScript`
  (`parent.UserConstructionScript`))