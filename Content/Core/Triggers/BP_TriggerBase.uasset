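; Base directional trigger that runs an overridable TriggerAction when the player pawn leaves its box.
; Comparing player distance to VisibilityPoint and InvisibilityPoint sets Forward, which raises or lowers the trigger count; reaching the limit disables overlap events, with -1 meaning unlimited.
; Each activation writes ID, count and direction to GravitySuperliminalPawn's TriggerState and prints debug text.
; ActivateFully and ActivatePartially replay activations without an overlap.
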(event `self.TriggerBox.OnComponentEndOverlap`
  (params (OverlappedComponent :type "PrimitiveComponent Object Reference") (OtherActor :type "Actor Object Reference") (OtherComp :type "PrimitiveComponent Object Reference") (OtherBodyIndex :type Integer))
  (if (== OtherActor (`GameplayStatics.GetPlayerPawn` 0))
    (`self.SetDirection`)
    (`self.ActivateTrigger`)))

(fn `ActivateFully`
  (bind _triggerlimit (`self.TriggerLimit`))
  (if (!= _triggerlimit -1)
    (for _ (range _triggerlimit)
      (`self.ActivateTrigger`))
    (else
      (`self.ActivateTrigger`))))

(fn `ActivatePartially`
  (params (Forward :type Boolean) (TriggerCount :type Integer))
  (if (!= (`self.TriggerLimit`) -1)
    (for _ (range TriggerCount)
      (`self.ActivateTrigger`))
    (else
      (set `self.Forward` Forward)
      (`self.ActivateTrigger`))))

(fn `ActivateTrigger`
  (bind _triggercount (`self.TriggerCount`))
  (bind _forward (`self.Forward`))
  (bind _id (`self.ID`))
  (`self.Trigger Action`)
  (`self.SetTriggerCount`)
  (bind _asgravity_superliminal_pawn (cast `/Game/Core/Pawns/GravitySuperliminalPawn` (`GameplayStatics.GetPlayerPawn` 0)))
  (set `/Game/Core/Pawns/GravitySuperliminalPawn.TriggerState` (make `/Game/Core/Triggers/STriggerState` _id _triggercount _forward) _asgravity_superliminal_pawn)
  (`KismetSystemLibrary.PrintString` (`KismetStringLibrary.Concat_StrStr` "Trigger " (`KismetStringLibrary.Conv_IntToString` _id) " activated " (`KismetStringLibrary.Conv_IntToString` _triggercount) " and is " (`KismetMathLibrary.SelectString` "forward" "backward" _forward))))

(fn `Hide`
  (set `PrimitiveComponent.bGenerateOverlapEvents` false (`self.TriggerBox`)))

(fn `SetDirection`
  (bind _returnvalue (`GameplayStatics.GetPlayerPawn` 0))
  (if (> (`KismetMathLibrary.Vector_Distance` (`SceneComponent.K2_GetComponentLocation` (`self.VisibilityPoint`)) (`self.K2_GetActorLocation` _returnvalue)) (`KismetMathLibrary.Vector_Distance` (`SceneComponent.K2_GetComponentLocation` (`self.InvisibilityPoint`)) (`self.K2_GetActorLocation` _returnvalue)))
    (set `self.Forward` true)
    (else
      (set `self.Forward` false))))

(fn `SetTriggerCount`
  (bind _triggercount (`self.TriggerCount`))
  (if (`self.Forward`)
    (`/Engine/EditorBlueprintResources/StandardMacros.IncrementInt` _triggercount
      (:`  `
        (if (and (>= (`self.TriggerCount`) (`self.TriggerLimit`)) (!= (`self.TriggerLimit`) -1)) :!label _label
          (`self.Hide`))))
    (elif (not (== _triggercount 0))
      (`/Engine/EditorBlueprintResources/StandardMacros.DecrementInt` _triggercount
        (:`  `
          (goto _label))))))

(fn `Show`
  (set `PrimitiveComponent.bGenerateOverlapEvents` true (`self.TriggerBox`)))

(fn `Trigger Action`)

(fn `UserConstructionScript`)