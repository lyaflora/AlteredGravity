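; BP_Niagara_Gravity is an actor that lets the player switch the gravity direction of its Niagara effect from the keyboard.
; It enables input from the first player controller on BeginPlay and listens for number keys 0 to 3.
; Each press converts the key's display name to an integer, stores it as SelectedGravityDirection and passes it to the Niagara component's User.GravityDirection parameter.
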(event `self.ReceiveBeginPlay`
  (`self.EnableInput` (`GameplayStatics.GetPlayerController` 0)))

(event `Key|Zero`
  (params (Key :type "Key Structure"))
  (:`Pressed`
    (set `self.SelectedGravityDirection` (`KismetStringLibrary.Conv_StringToInt` (`KismetTextLibrary.Conv_TextToString` (`KismetInputLibrary.Key_GetDisplayName` Key))))
    (`NiagaraComponent.SetVariableInt` (`self.NiagaraComponent`) "User.GravityDirection" (`self.SelectedGravityDirection`) :!label _label)))

(event `Key|One`
  (params (Key :type "Key Structure"))
  (:`Pressed`
    (set `self.SelectedGravityDirection` (`KismetStringLibrary.Conv_StringToInt` (`KismetTextLibrary.Conv_TextToString` (`KismetInputLibrary.Key_GetDisplayName` Key))))
    (goto _label)))

(event `Key|Two`
  (params (Key :type "Key Structure"))
  (:`Pressed`
    (set `self.SelectedGravityDirection` (`KismetStringLibrary.Conv_StringToInt` (`KismetTextLibrary.Conv_TextToString` (`KismetInputLibrary.Key_GetDisplayName` Key))))
    (goto _label)))

(event `Key|Three`
  (params (Key :type "Key Structure"))
  (:`Pressed`
    (set `self.SelectedGravityDirection` (`KismetStringLibrary.Conv_StringToInt` (`KismetTextLibrary.Conv_TextToString` (`KismetInputLibrary.Key_GetDisplayName` Key))))
    (goto _label)))

(fn `UserConstructionScript`)