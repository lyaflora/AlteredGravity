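; BP_Trigger_ShowHide is a trigger that swaps the visibility of two groups of controlled hideable objects.
; Its Trigger Action checks the Forward flag: when true it hides group A and shows group B, and when false it does the reverse.
; BeginPlay, the construction script and the trigger's own Show and Hide events only call the parent implementation.
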(event `self.ReceiveBeginPlay`
  (`parent.ReceiveBeginPlay`))

(event `self.Hide`
  (`parent.Hide`))

(event `self.Show`
  (`parent.Show`))

(fn `Trigger Action`
  (for _array_element (`self.ControlledHideablesA`)
    (if (`self.Forward`)
      (`self.Hide` _array_element)
      (else
        (`self.Show` _array_element))))
  (for _array_element_2 (`self.ControlledHideablesB`)
    (if (`self.Forward`)
      (`self.Show` _array_element_2)
      (else
        (`self.Hide` _array_element_2)))))

(fn `UserConstructionScript`
  (`parent.UserConstructionScript`))