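; Circle trigger Blueprint that toggles two groups of hideable objects in opposition as it is activated.
; TriggerAction uses direction and trigger count to step back and forth between two states: group A hidden with B shown, or the reverse.
; ActivatePartially reaches a given count and direction by replaying ActivateTrigger calls, while ActivateFully fires it twice.
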(fn `ActivateFully`
  (`self.ActivateTrigger`)
  (`self.ActivateTrigger`))

(fn `ActivatePartially`
  (params (Forward :type Boolean) (TriggerCount :type Integer))
  (for _ (range 1 (+ (`KismetMathLibrary.SelectInt` TriggerCount (+ TriggerCount 1) Forward) 1))
    (`self.ActivateTrigger`))
  (if (not Forward)
    (set `self.Forward` Forward)
    (`self.ActivateTrigger`)))

(fn `Trigger Action`
  (bind _triggercount (`self.TriggerCount`))
  (bind _triggercount_2 (`self.TriggerCount`))
  (for _array_element (`self.ControlledHideablesA`)
    (if (`self.Forward`)
      (switch `int` _triggercount
        (:`0`
          (`self.Hide` _array_element :!label _label))
        (:`1`
          (`self.Show` _array_element :!label _label_2)))
      (else
        (switch `int` _triggercount
          (:`1`
            (goto _label_2))
          (:`2`
            (goto _label))))))
  (for _array_element_2 (`self.ControlledHideablesB`)
    (if (`self.Forward`)
      (switch `int` _triggercount_2
        (:`0`
          (`self.Show` _array_element_2 :!label _label_3))
        (:`1`
          (`self.Hide` _array_element_2 :!label _label_4)))
      (else
        (switch `int` _triggercount_2
          (:`1`
            (goto _label_4))
          (:`2`
            (goto _label_3)))))))

(fn `UserConstructionScript`
  (`parent.UserConstructionScript`))