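; BP_TriggerHandler restores level trigger progress from a saved trigger state.
; LoadTriggerState gathers all BP_TriggerBase actors, sorts them by ID through a comparator, then replays them in order up to the saved TriggerID.
; Limited triggers repeat ActivateTrigger up to their limit, or to the saved count for the saved one.
; Others call ActivateFully, except the saved one, which calls ActivatePartially with saved direction and count.
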(fn `Load Trigger State`
  (params (TriggerState :type "/Game/Core/Triggers/STriggerState Structure"))
  (locals (Triggers :type "Array of /Game/Core/Triggers/BP_TriggerBase Object Reference"))
  (bind (_triggerid _triggercount _triggerforward) (break `/Game/Core/Triggers/STriggerState` TriggerState))
  (bind _outactors (`GameplayStatics.GetAllActorsOfClass` "/Game/Core/Triggers/BP_TriggerBase.BP_TriggerBase_C"))
  (bind _output_get (set `local.Triggers` _outactors))
  (`LowEntryExtendedStandardLibrary.SortObjectArrayDirectly` _output_get (`|CreateDelegate` :!event `Trigger ID Comparator`))
  (`KismetSystemLibrary.PrintString` (`KismetStringLibrary.Concat_StrStr` (`KismetStringLibrary.Conv_IntToString` _triggerid) " trigger with a count of " (`KismetStringLibrary.Conv_IntToString` _triggercount) " in direction of " (`KismetStringLibrary.Conv_BoolToString` _triggerforward)))
  (for _index (range (+ _triggerid 1))
    (bind _output (`|GetArrayItem` (`local.Triggers`) _index))
    (bind _triggerlimit (`/Game/Core/Triggers/BP_TriggerBase.TriggerLimit` _output))
    (if (> _triggerlimit 0)
      (bind _returnvalue (== (`/Game/Core/Triggers/BP_TriggerBase.ID` _output) _triggerid))
      (for _ (range (+ (`KismetMathLibrary.SelectInt` (- _triggercount 1) (- _triggerlimit 1) _returnvalue) 1))
        (`/Game/Core/Triggers/BP_TriggerBase.ActivateTrigger` _output))
      (elif _returnvalue
        (`/Game/Core/Triggers/BP_TriggerBase.ActivatePartially` _output _triggerforward _triggercount)
        (else
          (`/Game/Core/Triggers/BP_TriggerBase.ActivateFully` _output))))))

(fn `Trigger ID Comparator`
  (params (ObjectA :type "Object Object Reference") (ObjectB :type "Object Object Reference"))
  (returns (Result :type Boolean))
  (locals (ResultTemp :type Boolean))
  (bind _asbp_trigger_base (cast `/Game/Core/Triggers/BP_TriggerBase` ObjectA)
    (:`then`
      (bind _asbp_trigger_base_2 (cast `/Game/Core/Triggers/BP_TriggerBase` ObjectB)
        (:`then`
          (set `local.ResultTemp` (< (`/Game/Core/Triggers/BP_TriggerBase.ID` _asbp_trigger_base) (`/Game/Core/Triggers/BP_TriggerBase.ID` _asbp_trigger_base_2))))
        (:`CastFailed`
          (set `local.ResultTemp` false :!label _label))))
    (:`CastFailed`
      (goto _label)))
  (return (`local.ResultTemp`)))

(fn `UserConstructionScript`)