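; BP_Trigger_DoorCover is a trigger Blueprint that hides and shows groups of controlled hideables, named as a cover for doors.
; Its Trigger Action loops over three hideable arrays and uses the Forward flag to decide what changes.
; When Forward is true, group A hides and group C shows; when false, only group B hides.
; The event graph and construction script add no logic of their own.
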(fn `Trigger Action`
  (for _array_element (`self.ControlledHideablesA`)
    (if (`self.Forward`)
      (`self.Hide` _array_element)))
  (for _array_element_2 (`self.ControlledHideablesB`)
    (if (not (`self.Forward`))
      (`self.Hide` _array_element_2)))
  (for _array_element_3 (`self.ControlledHideablesC`)
    (if (`self.Forward`)
      (`self.Show` _array_element_3))))

(fn `UserConstructionScript`
  (`parent.UserConstructionScript`))