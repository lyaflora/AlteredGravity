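; Trigger that launches the gravity pawn along a fixed, near +Y direction with a widening vertigo FOV.
; Its trigger action toggles Tick and swaps the pawn's custom gravity and damping: none when forward, downward gravity and light damping when reversed.
; While active, Tick overwrites velocity and FOV each frame, both growing with the player's distance from the trigger.
; Hiding stops the Tick effect without restoring gravity or damping.
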(event `self.ReceiveTick`
  (params (DeltaSeconds :type "Float (single-precision)"))
  (bind _returnvalue (`GameplayStatics.GetPlayerPawn` 0))
  (bind _returnvalue_2 (`KismetMathLibrary.Vector_Distance` (`self.K2_GetActorLocation` _returnvalue) (`self.K2_GetActorLocation`)))
  (if (`self.bActivated`)
    (bind _asgravity_superliminal_pawn (cast `/Game/Core/Pawns/GravitySuperliminalPawn` _returnvalue))
    (set `MovementComponent.Velocity` (* (0.036 0.999 0.0) (`KismetMathLibrary.MapRangeClamped` _returnvalue_2 0.0 10000.0 500.0 5000.0)) (`CustomPawn.MovementComponent` _asgravity_superliminal_pawn))
    (`/Game/Core/Pawns/GravitySuperliminalPawn.Set Vertigo FOV manually` _asgravity_superliminal_pawn (`KismetMathLibrary.MapRangeClamped` _returnvalue_2 0.0 5000.0 90.0 150.0))))

(fn `Hide`
  (`parent.Hide`)
  (set `self.bActivated` false)
  (`self.SetActorTickEnabled` false))

(fn `Trigger Action`
  (bind _forward (`self.Forward`))
  (`self.SetActorTickEnabled` (`self.Forward`))
  (set `self.bActivated` (`self.Forward`))
  (bind _asgravity_superliminal_pawn (cast `/Game/Core/Pawns/GravitySuperliminalPawn` (`GameplayStatics.GetPlayerPawn` 0)))
  (set `CustomMovementComponent.CustomGravityInfo` (make `GravityInfo` 980.0 (`KismetMathLibrary.SelectVector` (0.0 0.0 0.0) (0.0 0.0 -1.0) _forward)) (`CustomPawn.MovementComponent` _asgravity_superliminal_pawn))
  (`PrimitiveComponent.SetLinearDamping` (`CustomPawn.CapsuleComponent` _asgravity_superliminal_pawn) (`KismetMathLibrary.SelectFloat` 0.0 0.15 _forward)))

(fn `UserConstructionScript`
  (`parent.UserConstructionScript`))