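; Teleport trigger that shifts the player pawn by a configurable local offset when fired in the forward direction.
; The Trigger Action function calls an event that waits one tick, then applies the offset as an unswept teleport.
; It can also unhide a sky sphere to reveal a starry sky.
; The full and partial activation functions only set the trigger count.
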(event `TriggerAction`
  (`KismetSystemLibrary.DelayUntilNextTick`)
  (`self.K2_AddActorLocalOffset` (`GameplayStatics.GetPlayerPawn` 0) (`self.TeleportOffset`) false true))

(fn `ActivateFully`
  (`self.SetTriggerCount`))

(fn `ActivatePartially`
  (params (Forward :type Boolean) (TriggerCount :type Integer))
  (`self.SetTriggerCount`))

(fn `Trigger Action`
  (if (`self.Forward`)
    (`self.TriggerAction`)
    (if (`self.bRevealStarrySky`)
      (`self.SetActorHiddenInGame` (`self.SkySphere`) false))))

(fn `UserConstructionScript`
  (`parent.UserConstructionScript`))