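; BP_Trigger_FakeDoor is a trigger that swaps the visibility of two sets of hideable objects, presumably to fake a door.
; Its TriggerAction hides the A set when Forward is true and shows the B set when it is false.
; Full activation fires the trigger backward then forward, showing B before hiding A.
; Partial activation always fires the backward pass and adds the forward pass only when requested.
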(fn `ActivateFully`
  (set `self.Forward` false)
  (`self.ActivateTrigger`)
  (set `self.Forward` true)
  (`self.ActivateTrigger`))

(fn `ActivatePartially`
  (params (Forward :type Boolean) (TriggerCount :type Integer))
  (set `self.Forward` false)
  (`self.ActivateTrigger`)
  (if Forward
    (set `self.Forward` true)
    (`self.ActivateTrigger`)))

(fn `Trigger Action`
  (for _array_element (`self.ControlledHideablesA`)
    (if (`self.Forward`)
      (`self.Hide` _array_element)))
  (for _array_element_2 (`self.ControlledHideablesB`)
    (if (not (`self.Forward`))
      (`self.Show` _array_element_2))))

(fn `UserConstructionScript`
  (`parent.UserConstructionScript`))