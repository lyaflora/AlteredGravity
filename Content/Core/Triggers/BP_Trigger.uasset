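; BP_Trigger is a directional trigger volume that counts passes and can switch itself off after a limit.
; On end overlap, it sets Forward for the player pawn by comparing distances to VisibilityPoint and InvisibilityPoint.
; Any actor's exit then raises or lowers TriggerCount using the last Forward value, never decrementing from zero.
; Show and Hide only toggle overlap events; a TriggerLimit of -1 means unlimited.
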(event `self.ReceiveBeginPlay`
  (if (`self.isVisibleOnStart`)
    (`self.Show`)
    (else
      (`self.Hide`))))

(event `self.TriggerBox.OnComponentEndOverlap`
  (params (OverlappedComponent :type "PrimitiveComponent Object Reference") (OtherActor :type "Actor Object Reference") (OtherComp :type "PrimitiveComponent Object Reference") (OtherBodyIndex :type Integer))
  (`self.TriggerActivated` OtherActor)
  (`self.SetTriggerCount`))

(event `TriggerActivated`
  (params (OverlappingActor :type "Actor Object Reference"))
  (bind _returnvalue (`GameplayStatics.GetPlayerPawn` 0))
  (if (== OverlappingActor _returnvalue)
    (if (> (`KismetMathLibrary.Vector_Distance` (`SceneComponent.K2_GetComponentLocation` (`self.VisibilityPoint`)) (`self.K2_GetActorLocation` _returnvalue)) (`KismetMathLibrary.Vector_Distance` (`SceneComponent.K2_GetComponentLocation` (`self.InvisibilityPoint`)) (`self.K2_GetActorLocation` _returnvalue)))
      (set `self.Forward` true)
      (else
        (set `self.Forward` false)))))

(event `SetTriggerCount`
  (bind _triggercount (`self.TriggerCount`))
  (if (`self.Forward`)
    (`/Engine/EditorBlueprintResources/StandardMacros.IncrementInt` _triggercount
      (:`  `
        (`KismetSystemLibrary.PrintString` (`KismetStringLibrary.Conv_IntToString` _triggercount) :!label _label)
        (if (and (>= (`self.TriggerCount`) (`self.TriggerLimit`)) (!= (`self.TriggerLimit`) -1))
          (`self.Hide`))))
    (elif (not (== _triggercount 0))
      (`/Engine/EditorBlueprintResources/StandardMacros.DecrementInt` _triggercount
        (:`  `
          (goto _label))))))

(fn `Hide`
  (set `PrimitiveComponent.bGenerateOverlapEvents` false (`self.TriggerBox`)))

(fn `Show`
  (set `PrimitiveComponent.bGenerateOverlapEvents` true (`self.TriggerBox`)))

(fn `UserConstructionScript`)