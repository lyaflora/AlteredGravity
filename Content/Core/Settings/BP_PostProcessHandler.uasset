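; Post-process settings handler that drives a PostProcessVolume from the player's Brightness and Gamma values.
; After a short delay on BeginPlay, it notifies AlteredGravityGameInstance of its spawn and binds to its settings-loaded event to refresh the volume.
; UpdateSettings maps both values to manual-metering exposure compensation and gamma, storing the result as DisplayedSettings.
; ApplySettings records AppliedSettings and reverse-maps them into both values before updating again.
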(event `self.ReceiveBeginPlay`
  (`KismetSystemLibrary.Delay` 0.2)
  (bind _asaltered_gravity_game_instance (cast `/Game/Core/GameInstance/AlteredGravityGameInstance` (`GameplayStatics.GetGameInstance`)))
  (`/Game/Core/GameInstance/AlteredGravityGameInstance.OnPostProcessHandlerSpawned` _asaltered_gravity_game_instance)
  (add `/Game/Core/GameInstance/AlteredGravityGameInstance.SettingsLoaded` _asaltered_gravity_game_instance (delegate `OnSettingsLoaded`)))

(event `OnSettingsLoaded`
  (`self.UpdateSettings`)
  (`self.ApplySettings` (`self.DisplayedSettings`)))

(fn `ApplySettings`
  (params (SettingsToApply :type "PostProcessSettings Structure"))
  (bind _output_get (set `self.AppliedSettings` SettingsToApply))
  (bind ((`ColorGamma` _colorgamma) (`AutoExposureBias` _autoexposurebias)) (break `PostProcessSettings` _output_get))
  (set `self.Gamma` (`KismetMathLibrary.MapRangeClamped` (`.W` (`KismetMathLibrary.BreakVector4` _colorgamma)) 0.0 2.0 0.0 1.0))
  (set `self.Brightness` (`KismetMathLibrary.MapRangeClamped` _autoexposurebias 0.0 20.0 0.0 1.0))
  (`self.UpdateSettings`))

(fn `ResetDefaults`
  (set `self.Brightness` 0.5)
  (set `self.Gamma` 0.5)
  (`self.UpdateSettings`))

(fn `SetBrightness`
  (params (Brightness :type "Float (single-precision)"))
  (set `self.Brightness` Brightness)
  (`self.UpdateSettings`))

(fn `SetGamma`
  (params (Gamma :type "Float (double-precision)"))
  (set `self.Gamma` Gamma)
  (`self.UpdateSettings`))

(fn `UpdateSettings`
  (bind _output_get (set `PostProcessVolume.Settings` (make `PostProcessSettings` :`AutoExposureMethod` "AEM_Manual" :`ColorGamma` (`KismetMathLibrary.MakeVector4` 1.0 1.0 1.0 (`KismetMathLibrary.MapRangeClamped` (`self.Gamma`) 0.0 1.0 0.0 2.0)) :`AutoExposureBias` (`KismetMathLibrary.MapRangeClamped` (`self.Brightness`) 0.0 1.0 0.0 20.0) :`AutoExposureMinBrightness` 1.0 :`AutoExposureMaxBrightness` 1.0) (`self.PostProcessVolume`)))
  (set `self.DisplayedSettings` _output_get))

(fn `UserConstructionScript`)