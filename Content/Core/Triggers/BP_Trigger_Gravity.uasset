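; BP_Trigger_Gravity is a trigger that changes how the player pawn's vertical orientation is determined, for both standing and falling.
; Its trigger action casts player 0 to GravitySuperliminalPawn and sets both orientation modes on its movement component to SurfaceNormal when Forward is true, otherwise GravityDirection.
; ActivateFully always sets both modes to GravityDirection.
; BeginPlay, overlap, tick and construction only call the parent.
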(event `self.ReceiveBeginPlay`
  (`parent.ReceiveBeginPlay`))

(event `self.ReceiveActorBeginOverlap`
  (params (OtherActor :type "Actor Object Reference"))
  (`parent.ReceiveActorBeginOverlap` OtherActor))

(event `self.ReceiveTick`
  (params (DeltaSeconds :type "Float (single-precision)"))
  (`parent.ReceiveTick` DeltaSeconds))

(fn `ActivateFully`
  (bind _asgravity_superliminal_pawn (cast `/Game/Core/Pawns/GravitySuperliminalPawn` (`GameplayStatics.GetPlayerPawn` 0)))
  (bind _movementcomponent (`CustomPawn.MovementComponent` _asgravity_superliminal_pawn))
  (set `CustomMovementComponent.StandingVerticalOrientation` "EVO_GravityDirection" _movementcomponent)
  (set `CustomMovementComponent.FallingVerticalOrientation` "EVO_GravityDirection" _movementcomponent))

(fn `Trigger Action`
  (bind _asgravity_superliminal_pawn (cast `/Game/Core/Pawns/GravitySuperliminalPawn` (`GameplayStatics.GetPlayerPawn` 0)))
  (if (`self.Forward`)
    (bind _movementcomponent (`CustomPawn.MovementComponent` _asgravity_superliminal_pawn))
    (set `CustomMovementComponent.StandingVerticalOrientation` "EVO_SurfaceNormal" _movementcomponent)
    (set `CustomMovementComponent.FallingVerticalOrientation` "EVO_SurfaceNormal" _movementcomponent)
    (else
      (set `CustomMovementComponent.StandingVerticalOrientation` "EVO_GravityDirection" _movementcomponent)
      (set `CustomMovementComponent.FallingVerticalOrientation` "EVO_GravityDirection" _movementcomponent))))

(fn `UserConstructionScript`
  (`parent.UserConstructionScript`))