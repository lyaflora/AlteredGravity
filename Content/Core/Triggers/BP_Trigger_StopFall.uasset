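; Trigger that ends the player's fall by halting the GravitySuperliminalPawn and restoring standard downward gravity.
; Overrides the parent's Trigger Action, casting player pawn 0 and stopping its movement immediately before resetting custom gravity.
; It also snaps the spring arm to a fixed world rotation, sets capsule linear damping, disables movement and manually sets the vertigo FOV.
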(fn `Trigger Action`
  (`parent.Trigger Action`)
  (bind _asgravity_superliminal_pawn (cast `/Game/Core/Pawns/GravitySuperliminalPawn` (`GameplayStatics.GetPlayerPawn` 0)))
  (bind _movementcomponent (`CustomPawn.MovementComponent` _asgravity_superliminal_pawn))
  (`MovementComponent.StopMovementImmediately` _movementcomponent)
  (set `CustomMovementComponent.CustomGravityInfo` (make `GravityInfo` 980.0) _movementcomponent)
  (`SceneComponent.K2_SetWorldRotation` (`CustomPawn.SpringArm` _asgravity_superliminal_pawn) (struct :`Pitch` -90.0 :`Yaw` 90.0) false true)
  (`PrimitiveComponent.SetLinearDamping` (`CustomPawn.CapsuleComponent` _asgravity_superliminal_pawn) 0.15)
  (set `/Game/Core/Pawns/GravitySuperliminalPawn.bMovementEnabled` false _asgravity_superliminal_pawn)
  (`/Game/Core/Pawns/GravitySuperliminalPawn.Set Vertigo FOV manually` _asgravity_superliminal_pawn 90.0))

(fn `UserConstructionScript`
  (`parent.UserConstructionScript`))