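; Trigger Blueprint that shows and hides four groups of hideables (A to D) as it steps through a two-stage, reversible sequence.
; TriggerAction uses Forward and TriggerCount to pick what changes in each group.
; The first forward step swaps A for B, and the second hides B and C and reveals D.
; Backward steps mirror these changes, restoring the earlier visibility.
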(fn `Trigger Action`
  (bind _triggercount (`self.TriggerCount`))
  (bind _triggercount_2 (`self.TriggerCount`))
  (bind _triggercount_3 (`self.TriggerCount`))
  (bind _triggercount_4 (`self.TriggerCount`))
  (for _array_element (`self.ControlledHideablesA`)
    (if (`self.Forward`)
      (switch `int` _triggercount
        (:`0`
          (`self.Hide` _array_element)))
      (else
        (switch `int` _triggercount
          (:`1`
            (`self.Show` _array_element))))))
  (for _array_element_2 (`self.ControlledHideablesB`)
    (if (`self.Forward`)
      (switch `int` _triggercount_2
        (:`0`
          (`self.Show` _array_element_2 :!label _label))
        (:`1`
          (`self.Hide` _array_element_2 :!label _label_2)))
      (else
        (switch `int` _triggercount_2
          (:`1`
            (goto _label_2))
          (:`2`
            (goto _label))))))
  (for _array_element_3 (`self.ControlledHideablesC`)
    (if (`self.Forward`)
      (switch `int` _triggercount_3
        (:`1`
          (`self.Hide` _array_element_3)))
      (else
        (switch `int` _triggercount_3
          (:`2`
            (`self.Show` _array_element_3))))))
  (for _array_element_4 (`self.ControlledHideablesD`)
    (if (`self.Forward`)
      (switch `int` _triggercount_4
        (:`1`
          (`self.Show` _array_element_4)))
      (else
        (switch `int` _triggercount_4
          (:`2`
            (`self.Hide` _array_element_4)))))))

(fn `UserConstructionScript`
  (`parent.UserConstructionScript`))