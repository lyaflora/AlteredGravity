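; BP_SurfaceGravityObject is an object whose GravityField volume makes a GravitySuperliminalPawn orient its vertical axis to surface normals.
; Entering the field switches the pawn movement component's standing and falling vertical orientations to SurfaceNormal.
; Leaving restores GravityDirection only when the pawn overlaps no other surface gravity object, so overlapping or adjacent fields hand off cleanly.
; Both overlap events print debug messages.
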(event `self.GravityField.OnComponentBeginOverlap`
  (params (OverlappedComponent :type "PrimitiveComponent Object Reference") (OtherActor :type "Actor Object Reference") (OtherComp :type "PrimitiveComponent Object Reference") (OtherBodyIndex :type Integer) (bFromSweep :type Boolean) (SweepResult :type "HitResult Structure (by ref)"))
  (bind _asgravity_superliminal_pawn (cast `/Game/Core/Pawns/GravitySuperliminalPawn` OtherActor))
  (bind _movementcomponent (`CustomPawn.MovementComponent` _asgravity_superliminal_pawn))
  (set `CustomMovementComponent.StandingVerticalOrientation` "EVO_SurfaceNormal" _movementcomponent)
  (set `CustomMovementComponent.FallingVerticalOrientation` "EVO_SurfaceNormal" _movementcomponent)
  (`KismetSystemLibrary.PrintString` "Gravity set to surface normal!"))

(event `self.GravityField.OnComponentEndOverlap`
  (params (OverlappedComponent :type "PrimitiveComponent Object Reference") (OtherActor :type "Actor Object Reference") (OtherComp :type "PrimitiveComponent Object Reference") (OtherBodyIndex :type Integer))
  (if (== (`KismetArrayLibrary.Array_Length` (`self.GetOverlappingActors` OtherActor "BP_SurfaceGravityObject_C")) 0)
    (bind _asgravity_superliminal_pawn (cast `/Game/Core/Pawns/GravitySuperliminalPawn` OtherActor))
    (bind _movementcomponent (`CustomPawn.MovementComponent` _asgravity_superliminal_pawn))
    (set `CustomMovementComponent.StandingVerticalOrientation` "EVO_GravityDirection" _movementcomponent)
    (set `CustomMovementComponent.FallingVerticalOrientation` "EVO_GravityDirection" _movementcomponent)
    (`KismetSystemLibrary.PrintString` "Gravity set to directional gravity!")))

(fn `UserConstructionScript`)